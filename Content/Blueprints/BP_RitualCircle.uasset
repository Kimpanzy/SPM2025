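; Ritual circle puzzle that ends the game: artifacts tagged 1–4 in slots A–D plus a caged rat pause play and show credits.
; Interaction picks the slot from the hit component name's last letter, then grabs or places via the player's Grabber.
; Each slot change or rat capture requests a save and solution check; slot artifact IDs persist as GUIDs.
; Tick flickers lightning planes by swapping two textures on dynamic materials at random intervals.
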(event `self.ReceiveBeginPlay`
  (bind _asrequiem_game_instance (cast `RequiemGameInstance` (`GameplayStatics.GetGameInstance`))
    (:`then`
      (`Persistence.RequestLoad` _asrequiem_game_instance self))
    (:`CastFailed`
      _))
  (bind _asbp_player (cast `/Game/Blueprints/BP_Player` (`GameplayStatics.GetPlayerPawn` 0)))
  (set `self.Grabber` (`/Game/Blueprints/BP_Player.Grabber` _asbp_player))
  (bind _asbp_rat_cage (cast `/Game/Rat/BP_RatCage` (`ChildActorComponent.ChildActor` (`self.ChildActor`))))
  (bind _output_get (set `self.As BP Rat Cage` _asbp_rat_cage))
  (add `/Game/Rat/BP_RatCage.RatCaged` _output_get (delegate `RatCaged`))
  (`KismetArrayLibrary.Array_Add` (`self.Planes`) (`self.Plane`))
  (`KismetArrayLibrary.Array_Add` (`self.Planes`) (`self.Plane1`))
  (`KismetArrayLibrary.Array_Add` (`self.Planes`) (`self.Plane2`))
  (`KismetArrayLibrary.Array_Add` (`self.Planes`) (`self.Plane3`))
  (`KismetArrayLibrary.Array_Add` (`self.Planes`) (`self.Plane4`))
  (`KismetArrayLibrary.Array_Add` (`self.Planes`) (`self.Plane5`))
  (`KismetArrayLibrary.Array_Add` (`self.Planes`) (`self.Plane6`))
  (`KismetArrayLibrary.Array_Add` (`self.Planes`) (`self.Plane7`))
  (`KismetArrayLibrary.Array_Add` (`self.Planes`) (`self.Plane8`))
  (`KismetArrayLibrary.Array_Add` (`self.Planes`) (`self.Plane9`))
  (for _array_element (`self.Planes`)
    (bind _returnvalue (`KismetMaterialLibrary.CreateDynamicMaterialInstance` "/Game/Assets/Textures/Lightning.Lightning"))
    (bind _output_get_2 (set `self.Mat` _returnvalue))
    (`PrimitiveComponent.SetMaterial` _array_element 0 _output_get_2)
    (bind _asmaterial_instance_dynamic (cast `MaterialInstanceDynamic` (`PrimitiveComponent.GetMaterial` _array_element 0)))
    (`KismetArrayLibrary.Array_Add` (`self.Mats`) (make `/Game/LightningQueue` _asmaterial_instance_dynamic (`KismetMathLibrary.RandomFloatInRange` 0.01 0.15)))))

(event `RatCaged`
  (bind _asrequiem_game_instance (cast `RequiemGameInstance` (`GameplayStatics.GetGameInstance`) :!label _label))
  (`Persistence.RequestSave` _asrequiem_game_instance true)
  (`self.CheckForSolution`))

(event `self.OnInteract`
  (params (HitResult :type "HitResult Structure"))
  (bind _returnvalue (`KismetSystemLibrary.GetDisplayName` (`.HitComponent` (`GameplayStatics.BreakHitResult` HitResult))))
  (bind _returnvalue_2 (`KismetStringLibrary.Len` _returnvalue))
  (bind _returnvalue_3 (`KismetStringLibrary.GetSubstring` _returnvalue (- _returnvalue_2 1) _returnvalue_2))
  (if (`KismetStringLibrary.EqualEqual_StrStr` _returnvalue_3 "A")
    (bind _slotobjectreturn (`self.GrabOrPlace` (`self.SlotAObject`) (`self.SlotA`)))
    (set `self.SlotAObject` _slotobjectreturn)
    (goto _label)
    (elif (`KismetStringLibrary.EqualEqual_StrStr` _returnvalue_3 "B")
      (bind _slotobjectreturn_2 (`self.GrabOrPlace` (`self.SlotBObject`) (`self.SlotB`)))
      (set `self.SlotBObject` _slotobjectreturn_2)
      (goto _label)
      (elif (`KismetStringLibrary.EqualEqual_StrStr` _returnvalue_3 "C")
        (bind _slotobjectreturn_3 (`self.GrabOrPlace` (`self.SlotCObject`) (`self.SlotC`)))
        (set `self.SlotCObject` _slotobjectreturn_3)
        (goto _label)
        (elif (`KismetStringLibrary.EqualEqual_StrStr` _returnvalue_3 "D")
          (bind _slotobjectreturn_4 (`self.GrabOrPlace` (`self.SlotDObject`) (`self.SlotD`)))
          (set `self.SlotDObject` _slotobjectreturn_4)
          (goto _label))))))

(event `self.SaveData`
  (params (SaveGameInstance :type "RequiemSaveGame Object Reference"))
  (bind _ritualcircle_slotobjectids (break `RitualCircleSaveData` (`RequiemSaveGame.RitualCircle` SaveGameInstance)))
  (bind _array (`|MakeArray` (`self.SlotAObject`) (`self.SlotBObject`) (`self.SlotCObject`) (`self.SlotDObject`)))
  (`KismetArrayLibrary.Array_Resize` _ritualcircle_slotobjectids (`KismetArrayLibrary.Array_Length` _array))
  (for (_array_element _array_index) _array
    (bind _asbp_artifact (cast `/Game/Blueprints/BP_Artifact` _array_element))
    (`KismetArrayLibrary.Array_Set` _ritualcircle_slotobjectids _array_index (`/Game/Blueprints/BP_Artifact.ID` _asbp_artifact))))

(event `self.LoadData`
  (params (SaveGameInstance :type "RequiemSaveGame Object Reference"))
  (bind _ritualcircle_slotobjectids (break `RitualCircleSaveData` (`RequiemSaveGame.RitualCircle` SaveGameInstance)))
  (bind _outactors (`GameplayStatics.GetAllActorsOfClass` "/Game/Blueprints/BP_Artifact.BP_Artifact_C"))
  (for (_array_element _array_index) _ritualcircle_slotobjectids
    (if (`KismetGuidLibrary.IsValid_Guid` _array_element)
      (for _array_element_2 _outactors
        (if (== (`/Game/Blueprints/BP_Artifact.ID` _array_element_2) _array_element)
          (switch `int` _array_index
            (:`0`
              (set `self.SlotAObject` _array_element_2))
            (:`1`
              (set `self.SlotBObject` _array_element_2))
            (:`2`
              (set `self.SlotCObject` _array_element_2))
            (:`3`
              (set `self.SlotDObject` _array_element_2))))))))

(event `self.ReceiveTick`
  (params (DeltaSeconds :type "Float (single-precision)"))
  (for (_array_element _array_index) (`self.Mats`)
    (bind (_mat _timetoswap) (break `/Game/LightningQueue` _array_element))
    (bind _returnvalue (- _timetoswap (* DeltaSeconds 0.7)))
    (`KismetSystemLibrary.PrintString` (`KismetStringLibrary.Conv_DoubleToString` _returnvalue))
    (if (<= _returnvalue 0.0)
      (bind _returnvalue_2 (`MaterialInstanceDynamic.K2_GetTextureParameterValue` _mat "LightningImage"))
      (if (== _returnvalue_2 "/Game/Assets/Textures/lightningframe1.lightningframe1")
        (`MaterialInstanceDynamic.SetTextureParameterValue` _mat "LightningImage" "/Game/Assets/Textures/lightningframe2.lightningframe2")
        (`KismetSystemLibrary.PrintString` "Hello")
        (else
          (`MaterialInstanceDynamic.SetTextureParameterValue` _mat "LightningImage" "/Game/Assets/Textures/lightningframe1.lightningframe1")))
      (bind _structout (setmembers `/Game/LightningQueue` :`StructRef` _array_element :`TimeToSwap` (`KismetMathLibrary.RandomFloatInRange` 0.05 0.2)))
      (`KismetArrayLibrary.Array_Set` (`self.Mats`) _array_index _structout)
      (else
        (bind _structout_2 (setmembers `/Game/LightningQueue` :`StructRef` _array_element :`TimeToSwap` _returnvalue))
        (`KismetArrayLibrary.Array_Set` (`self.Mats`) _array_index _structout_2)))))

(fn `CheckForSolution`
  (if (and (`KismetSystemLibrary.IsValid` (`self.SlotAObject`)) (`KismetSystemLibrary.IsValid` (`self.SlotBObject`)) (`KismetSystemLibrary.IsValid` (`self.SlotCObject`)) (`KismetSystemLibrary.IsValid` (`self.SlotDObject`)))
    (if (and (`/Game/Rat/BP_RatCage.RatIsInCage` (`self.As BP Rat Cage`)) (`self.ActorHasTag` (`self.SlotAObject`) "1") (`self.ActorHasTag` (`self.SlotBObject`) "2") (`self.ActorHasTag` (`self.SlotCObject`) "3") (`self.ActorHasTag` (`self.SlotDObject`) "4"))
      (`GameplayStatics.SetGamePaused` true)
      (bind _returnvalue (`|CreateWidget` "/Game/Blueprints/Menu_Widgets/WBP_Credits.WBP_Credits_C"))
      (`UserWidget.AddToViewport` _returnvalue 0)
      (set `PlayerController.bShowMouseCursor` true (`GameplayStatics.GetPlayerController` 0)))))

(fn `GetInteractPrompt`
  (params (HitResult :type "HitResult Structure"))
  (returns (ReturnValue :type Text))
  (locals (ReturnText :type Text))
  (bind _returnvalue (`KismetSystemLibrary.GetDisplayName` (`.HitComponent` (`GameplayStatics.BreakHitResult` HitResult))))
  (bind _returnvalue_2 (`KismetStringLibrary.Len` _returnvalue))
  (bind _returnvalue_3 (`KismetStringLibrary.GetSubstring` _returnvalue (- _returnvalue_2 1) _returnvalue_2))
  (if (`KismetStringLibrary.EqualEqual_StrStr` _returnvalue_3 "A")
    (bind _returntext1 (`self.GrabOrPlacePrompt` (`self.SlotAObject`)))
    (set `local.ReturnText` _returntext1)
    (elif (`KismetStringLibrary.EqualEqual_StrStr` _returnvalue_3 "B")
      (bind _returntext1_2 (`self.GrabOrPlacePrompt` (`self.SlotBObject`)))
      (set `local.ReturnText` _returntext1_2)
      (elif (`KismetStringLibrary.EqualEqual_StrStr` _returnvalue_3 "C")
        (bind _returntext1_3 (`self.GrabOrPlacePrompt` (`self.SlotCObject`)))
        (set `local.ReturnText` _returntext1_3)
        (elif (`KismetStringLibrary.EqualEqual_StrStr` _returnvalue_3 "D")
          (bind _returntext1_4 (`self.GrabOrPlacePrompt` (`self.SlotDObject`)))
          (set `local.ReturnText` _returntext1_4)
          (elif (`KismetStringLibrary.EqualEqual_StrStr` _returnvalue_3 "E")
            (bind _returntext1_5 (`self.GrabOrPlacePrompt` null))
            (set `local.ReturnText` _returntext1_5)
            (else
              (set `local.ReturnText` "")))))))
  (return (`local.ReturnText`)))

(fn `GrabOrPlace`
  (params (SlotObject :type "Actor Object Reference") (Slot :type "BoxComponent Object Reference"))
  (returns (SlotObjectReturn :type "Actor Object Reference"))
  (locals (ReturnObject :type "Actor Object Reference"))
  (bind _grabber (`self.Grabber`))
  (set `local.ReturnObject` SlotObject)
  (if (`KismetSystemLibrary.IsValid` (`local.ReturnObject`))
    (if (not (`KismetSystemLibrary.IsValid` (`Grabber.GrabbedActor` (`self.Grabber`))))
      (`Grabber.Grab` :`self` (`self.Grabber`) :`HitActor` (`local.ReturnObject`))
      (set `local.ReturnObject` null)
      (return (`local.ReturnObject`)))
    (else
      (set `local.ReturnObject` (`Grabber.GrabbedActor` _grabber))
      (`Grabber.ReleaseAtPos` :`self` _grabber :`Location` (+ (`SceneComponent.K2_GetComponentLocation` Slot) (0.0 0.0 0.0)))
      (return (`local.ReturnObject`)))))

(fn `GrabOrPlacePrompt`
  (params (SlotObj :type "Actor Object Reference"))
  (returns (ReturnText1 :type Text))
  (locals (ReturnString :type Text))
  (if (`KismetSystemLibrary.IsValid` SlotObj)
    (if (`KismetSystemLibrary.IsValid` (`Grabber.GrabbedActor` (`self.Grabber`)))
      (set `local.ReturnString` "Already Holding Item")
      (else
        (set `local.ReturnString` "Grab")))
    (elif (`KismetSystemLibrary.IsValid` (`Grabber.GrabbedActor` (`self.Grabber`)))
      (if (not (`self.ActorHasTag` (`Grabber.GrabbedActor` (`self.Grabber`)) "Rat"))
        (set `local.ReturnString` "Place")
        (else
          (set `local.ReturnString` "" :!label _label)))
      (else
        (goto _label))))
  (return (`local.ReturnString`)))

(fn `UserConstructionScript`)