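; KeyDoor is an interactable double door that opens when the player holds its required key, with a prompt reflecting key possession.
; Interacting plays a sound and opens every KeyDoor sharing that key.
; OpenDoor swings both meshes via a Timeline rotation lerp, then disables their collision.
; On finish, Yellow or Red doors unlock a matching path on the NPC possessed by the player's AIController reference.
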(event `OpenDoor`
  (set `self.IsOpen` true)
  (bind (_direction _height) (`Timeline|Timeline`)
    (:`Update`
      (`|ExecutionSequence`
        (:`then_0`
          (`SceneComponent.K2_SetRelativeRotation` (`self.SM_Door1`) (`KismetMathLibrary.RLerp` (struct :`Yaw` -180.0) (struct :`Yaw` -260.0) _height) false false))
        (:`then_1`
          (`SceneComponent.K2_SetRelativeRotation` (`self.SM_Door`) (`KismetMathLibrary.RLerp` (struct :`Yaw` -180.0) (struct :`Yaw` -100.0) _height) false false))))
    (:`Finished`
      (`PrimitiveComponent.SetCollisionEnabled` (`self.SM_Door1`) "NoCollision")
      (`PrimitiveComponent.SetCollisionEnabled` (`self.SM_Door`) "NoCollision")
      (bind _asbp_player (cast `/Game/Blueprints/BP_Player` (`GameplayStatics.GetPlayerCharacter` 0)))
      (bind _asbp_npc (cast `/Game/AI/BP_NPC` (`Controller.K2_GetPawn` (`PlayerCharacter.AIController` _asbp_player))))
      (if (`KismetStringLibrary.EqualEqual_StrStr` (`self.RequiredKey`) "Yellow")
        (bind _allpaths (`NPC.AllPaths` _asbp_npc))
        (`NPC.UnlockPath` _asbp_npc (`|GetArrayItem` _allpaths 1))
        (elif (`KismetStringLibrary.EqualEqual_StrStr` (`self.RequiredKey`) "Red")
          (`NPC.UnlockPath` _asbp_npc (`|GetArrayItem` _allpaths 2)))))))

(event `self.OnInteract`
  (params (HitResult :type "HitResult Structure"))
  (bind _asbp_player (cast `/Game/Blueprints/BP_Player` (`GameplayStatics.GetPlayerCharacter` 0)))
  (if (and (`KismetArrayLibrary.Array_Contains` (`/Game/Blueprints/BP_Player.Keys` _asbp_player) (`self.RequiredKey`)) (not (`self.IsOpen`)))
    (`self.OpenDoor`)
    (`GameplayStatics.PlaySound2D` "/Game/GameAudio/Foleys_SFX/A_DoorOpening.A_DoorOpening" 1.0 1.0 0.0 null null)
    (bind _outactors (`GameplayStatics.GetAllActorsOfClass` "KeyDoor_C"))
    (for _array_element _outactors
      (if (`KismetStringLibrary.EqualEqual_StrStr` (`/Game/Blueprints/KeyDoor.RequiredKey` _array_element) (`self.RequiredKey`))
        (`self.OpenDoor` _array_element)))))

(fn `GetInteractPrompt`
  (params (HitResult :type "HitResult Structure"))
  (returns (ReturnValue :type Text))
  (bind _asbp_player (cast `/Game/Blueprints/BP_Player` (`GameplayStatics.GetPlayerCharacter` 0)))
  (if (not (`self.IsOpen`))
    (if (`KismetArrayLibrary.Array_Contains` (`/Game/Blueprints/BP_Player.Keys` _asbp_player) (`self.RequiredKey`))
      (return "Use Key")
      (else
        (return (`KismetTextLibrary.Conv_StringToText` (`KismetStringLibrary.Concat_StrStr` "Need " (`self.RequiredKey`) " Key")))))
    (else
      (return ""))))

(fn `UserConstructionScript`)