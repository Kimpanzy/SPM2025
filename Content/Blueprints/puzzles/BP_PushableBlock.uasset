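; Pushable puzzle block that the player character shoves a fixed distance along the X or Y axis by walking into it.
; On hit, it snaps the player-to-block direction to the dominant axis, then checks that the player faces the block and a block-sized box trace is clear.
; A timeline then slides the block with the player attached and movement disabled, restoring walking when finished.
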(event Custom|Push
  (Variables|Default|SetPushing%20From (Transformation|GetActorLocation))
  (Variables|Default|SetPushing true)
  (bind _position (Timeline|MoveBlock PlayFromStart)
    (:Update
      (Transformation|SetActorRelativeLocation (|(((Direction*Length)*Position)+From) (Variables|Default|GetPushing%20From) (Variables|Default|GetPushableDirection) (Variables|Default|GetPush%20Length) _position)))
    (:Finished
      (CallFunction|StopPushing))))

(event Custom|StopPushing
  (bind _returnvalue (Game|GetPlayerCharacter 0))
  (Variables|Default|SetPushing false)
  (Transformation|DetachFromActor _returnvalue "KeepWorld" "KeepWorld" "KeepWorld")
  (Pawn|Components|CharacterMovement|SetMovementMode (Variables|/Script/Engine.Character|GetCharacterMovement _returnvalue) "MOVE_Walking" 0))

(event EventBeginPlay)

(event Collision|EventActorBeginOverlap
  (params (OtherActor :type Actor%20Object%20Reference)))

(event EventTick
  (params (DeltaSeconds :type Float%20%28single-precision%29)))

(event Collision|EventHit
  (params (MyComp :type Primitive%20Component%20Object%20Reference) (Other :type Actor%20Object%20Reference) (OtherComp :type Primitive%20Component%20Object%20Reference) (bSelfMoved :type Boolean) (HitLocation :type Vector :default "0, 0, 0") (HitNormal :type Vector :default "0, 0, 0") (NormalImpulse :type Vector :default "0, 0, 0") (Hit :type Hit%20Result%20Structure%20%28by%20ref%29))
  (bind _returnvalue (Game|GetPlayerCharacter 0))
  (if (== Other _returnvalue)
    (bind _direction_vector (CallFunction|AxisDirection (CallFunction|GetVectorBetween self _returnvalue)))
    (if (CallFunction|CanPush _returnvalue _direction_vector)
      (Variables|Default|SetPushableDirection _direction_vector)
      (Pawn|Components|CharacterMovement|DisableMovement (Variables|/Script/Engine.Character|GetCharacterMovement _returnvalue))
      (Transformation|AttachActorToActor _returnvalue self "None" "KeepWorld" "KeepWorld" "KeepWorld" false)
      (CallFunction|Push))))

(fn ConstructionScript)

(fn CanPush
  (params (Pusher :type Actor%20Object%20Reference) (Direction :type Vector))
  (bind _returnvalue (Transformation|GetActorLocation))
  (bind _cube (Variables|Default|GetCube))
  (if (Math|Boolean|ANDBoolean (not (Variables|Default|GetPushing)) (Utilities|Operators|NotEqual(!=) :A Direction :ErrorTolerance 0.0001) (<= (CallFunction|Anglefrom Pusher) 2e+01))
    (bind _returnvalue_2 (Class|KismetSystemLibrary|BoxTraceMulti _returnvalue (|(ActorLocation+(Direction*Length)) _returnvalue Direction (Variables|Default|GetPush%20Length)) (- (* (Variables|/Script/Engine.SceneComponent|GetRelativeScale3D _cube) (.boxextent (StaticMesh|GetBounds (Variables|/Script/Engine.StaticMeshComponent|GetStaticMesh _cube)))) "0.000100,0.000100,0.000100") "0, 0, 0" "TraceTypeQuery1" false (Utilities|Array|MakeArray self) "ForDuration" true))
    (return (not _returnvalue_2))
    (else
      (return false))))

(fn GetVectorBetween
  (params (Actor1 :type Actor%20Object%20Reference%20%28by%20ref%29) (Actor2 :type Actor%20Object%20Reference%20%28by%20ref%29))
  (return (Math|Vector2D|Normalize2D (Math|Conversions|ToVector2D(Vector) (- (Transformation|GetActorLocation Actor1) (Transformation|GetActorLocation Actor2))))))

(fn RoundVector
  (params (Vector :type Vector))
  (return (Math|Vector|MakeVector (Math|Conversions|ToFloat(Integer) (Math|Float|Round (.x Vector))) (Math|Conversions|ToFloat(Integer) (Math|Float|Round (.y Vector))) (Math|Conversions|ToFloat(Integer) (Math|Float|Round (.z Vector))))))

(fn Anglefrom
  (params (Pusher :type Actor%20Object%20Reference))
  (bind _returnvalue (Transformation|GetActorForwardVector Pusher))
  (bind _self self)
  (bind _vectorbetween (CallFunction|GetVectorBetween Pusher _self))
  (bind _returnvalue_2 (Math|Conversions|ToVector2D(Vector) _returnvalue))
  (return (|(180-(ABS((dot*signCross)))) (Class|KismetMathLibrary|DegAcos (Math|Vector2D|DotProduct(2D) _returnvalue_2 _vectorbetween)) (Math|Float|Sign(Float) (Class|KismetMathLibrary|CrossProduct2D _returnvalue_2 _vectorbetween)))))

(fn AxisDirection
  (params (Direction :type Vector%202D%20Structure))
  (if (|((ABS(X))>(ABS(Y))) (.x Direction) (.y Direction))
    (return (Math|Vector|MakeVector (Math|Conversions|ToFloat(Integer) (Math|Float|Round (.x Direction))) 0.0 0.0))
    (else
      (return (Math|Vector|MakeVector 0.0 (Math|Conversions|ToFloat(Integer) (Math|Float|Round (.y Direction))) 0.0)))))