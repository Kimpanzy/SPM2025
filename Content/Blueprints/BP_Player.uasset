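; Player character for a stealth horror game with sprinting, breath holding, hiding, interaction, flashlight shake-recharging and saved progress.
; Heart rate from the heartbeat widget caps stamina, gates breath holding and sets idle noise range, while sprinting and recharging raise it.
; Movement, recharging and failed minigames report noise for AI, and failure also forces the player out of hiding.
; Tick drives noise, camera shake, stamina and trace-based prompts, while a looping timer eases FOV.
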(event OnComponentBeginOverlap(CapsuleComponent)
  (params (OverlappedComponent :type Primitive%20Component%20Object%20Reference) (OtherActor :type Actor%20Object%20Reference) (OtherComp :type Primitive%20Component%20Object%20Reference) (OtherBodyIndex :type Integer) (bFromSweep :type Boolean) (SweepResult :type Hit%20Result%20Structure%20%28by%20ref%29))
  (bind _asbp_npc (Utilities|Casting|CastToBP_NPC OtherActor))
  (if (not (Variables|Default|GetbIsHiding))
    (Class|CombatInterface|MeleeAttack _asbp_npc)))

(event Custom|InteractPrompt
  (bind _cameracomponent (Variables|Default|GetCameraComponent))
  (bind _returnvalue (Transformation|GetWorldLocation _cameracomponent))
  ;[0.15 0.15 0.15 0.5] Interact system
  (if (Utilities|IsValid (Variables|/Script/SPM2025.Grabber|GetGrabbedActor (Variables|Default|GetGrabber)))
    _
    (else
      _))
  (bind _outhit (Collision|SphereTraceByChannel _returnvalue (+ _returnvalue (* (Math|Vector|GetForwardVector (Transformation|GetWorldRotation _cameracomponent)) 1.8e+02)) 1e+01 "TraceTypeQuery3" false 0 "None"))
  (if (.bBlockingHit (Collision|BreakHitResult _outhit))
    (if (Actor|ActorHasTag (.HitActor (Collision|BreakHitResult _outhit)) "Interactable")
      (if (not (and (Actor|ActorHasTag (.HitActor (Collision|BreakHitResult _outhit)) "Grabbable") (Utilities|IsValid (Variables|/Script/SPM2025.Grabber|GetGrabbedActor (Variables|Default|GetGrabber)))))
        (bind _asinteractable (Utilities|Casting|CastToInteractable (.HitActor (Collision|BreakHitResult _outhit))))
        (bind _returnvalue_2 (Class|Interactable|GetInteractPrompt _asinteractable _outhit))
        (Variables|Default|SetInteractDisplay _returnvalue_2)
        (else
          (Variables|Default|SetInteractDisplay "Already Holding Item"))))
    (else
      (Variables|Default|SetInteractDisplay ""))))

(event Custom|SetSpeed
  (params (Multiplier :type Float%20%28double-precision%29))
  ;[0.15 0.15 0.15 0.5] Player speed related code
  (Variables|/Script/Engine.CharacterMovementComponent|SetMaxWalkSpeed (Variables|Character|GetCharacterMovement) (* Multiplier (Variables|Default|GetDefaultSpeed))))

(event Custom|HoldBreathTutorial
  (bind _newtrack_0 (Timeline|Timeline_1 PlayFromStart)
    (:Update
      (Widget|SetRenderOpacity (Variables|/Game/Blueprints/InGame_Widgets/WBP_MainUI.WBP_MainUI_C|GetHoldbreathTutorial (Variables|Default|GetMainUI)) _newtrack_0))
    (:Finished
      (Utilities|FlowControl|Delay 3.0)
      (bind _newtrack_0_2 (Timeline|Timeline_2 ReverseFromEnd)
        (:Update
          (Widget|SetRenderOpacity (Variables|/Game/Blueprints/InGame_Widgets/WBP_MainUI.WBP_MainUI_C|GetHoldbreathTutorial (Variables|Default|GetMainUI)) _newtrack_0_2))))))

(event Custom|MingameWinner
  (Utilities|FlowControl|Delay 4.0)
  (Variables|Default|SetCanExitHidingSpot true))

(event Custom|ReleaseYourBreath
  ;[0.15 0.15 0.15 0.5] Hold breath input
  (CallFunction|SetSpeed 1.0)
  (Variables|Default|SetTargetFOV 9e+01)
  (Variables|Default|SetIsHoldingBreath false)
  (Variables|Default|SetIsSprinting false)
  (Variables|Default|SetCanRegen true)
  (Variables|/Game/Blueprints/InGame_Widgets/WBP_HoldBreathVFX.WBP_HoldBreathVFX_C|SetTargetVignette (Variables|Default|GetHoldBreathUI) 0.0))

(event Custom|OnDeathEvent
  (params (Killer :type Actor%20Object%20Reference))
  (Default|DeathScreenEvent (Variables|Default|GetMainUI))
  (Audio|PlaySound2D "/Game/VA_Audio/Player_Audio/ScreamSoundCue.ScreamSoundCue" 1.0 1.0 0.0 0 0)
  (Utilities|FlowControl|Delay 1.5)
  (Game|OpenLevel(byObjectReference) "/Game/GameOver.GameOver"))

(event Custom|StaminaCooldown
  ;[0.15 0.15 0.15 0.5] Player speed related code
  (Variables|Default|SetCanRegen true))

(event Custom|FailedMinigame
  (CallFunction|ExitLocker)
  (Class|AISenseHearing|ReportNoiseEvent (Transformation|GetActorLocation) 1.0 self 5e+02 "None")
  (Audio|PlaySound2D "/Game/Assets/Sounds/forced_to_relase.forced_to_relase" 0.25 0.95 0.0 0 0))

(event Custom|ResetShakeCooldown
  (Variables|Default|SetCanShake true))

(event Custom|StartTutorial
  ;[0.15 0.15 0.15 0.5] Tutorial
  (bind _newtrack_0 (Timeline|Timeline Play)
    (:Update
      (Widget|SetRenderOpacity (Variables|/Game/Blueprints/InGame_Widgets/WBP_MainUI.WBP_MainUI_C|GetFlashlightTutorial (Variables|Default|GetMainUI)) _newtrack_0))))

(event Custom|SprintTutorial
  (bind _newtrack_0 (Timeline|Timeline_3 PlayFromStart)
    (:Update
      (Widget|SetRenderOpacity (Variables|/Game/Blueprints/InGame_Widgets/WBP_MainUI.WBP_MainUI_C|GetShiftTutorial (Variables|Default|GetMainUI)) _newtrack_0))
    (:Finished
      (Utilities|FlowControl|Delay 4.0)
      (bind _newtrack_0_2 (Timeline|Timeline_4 ReverseFromEnd)
        (:Update
          (Widget|SetRenderOpacity (Variables|/Game/Blueprints/InGame_Widgets/WBP_MainUI.WBP_MainUI_C|GetShiftTutorial (Variables|Default|GetMainUI)) _newtrack_0_2))))))

(event Input|EnhancedActionEvents|EnhancedInputActionIA_Sprint
  (params (ActionValue :type Boolean) (ElapsedSeconds :type Float%20%28double-precision%29) (TriggeredSeconds :type Float%20%28double-precision%29) (InputAction :type Input%20Action%20Object%20Reference :default "/Game/Inputs/IA_Sprint.IA_Sprint"))
  ;[0.15 0.15 0.15 0.5] Player speed related code
  (:Started
    (if (Math|Boolean|ANDBoolean (not false) (not (Variables|Default|GetIsHoldingBreath)) (> (Variables|Default|GetStamina) 0.0) (> (Math|Vector|VectorLength (Transformation|GetVelocity)) 1.0))
      (CallFunction|SetSpeed 2.0)
      (Variables|Default|SetIsSprinting true)
      (Audio|Components|Audio|Play (Variables|Default|GetFootstepsSprint) 0.0)
      (Utilities|Time|ClearandInvalidateTimerbyHandle (Variables|Default|GetHandle))
      (bind _howmuchchanged (Default|ChangeBPM (Variables|Default|GetHeartRateUI) 10 false))
      (Variables|Default|SetDecreaseByThisMuch _howmuchchanged)))
  (:Completed
    (if (Variables|Default|GetIsSprinting)
      (CallFunction|SetSpeed 1.0)
      (Audio|Components|Audio|Stop (Variables|Default|GetFootstepsSprint))
      (Variables|Default|SetIsSprinting false)
      (Variables|Default|SetCanRegen false)
      (bind _returnvalue (Utilities|Time|SetTimerbyFunctionName 0 "StaminaCooldown" 0.5))
      (Variables|Default|SetHandle _returnvalue)
      (Default|ChangeBPM (Variables|Default|GetHeartRateUI) (* (Variables|Default|GetDecreaseByThisMuch) -1) false))))

(event Input|EnhancedActionEvents|EnhancedInputActionIA_Interact
  (params (ActionValue :type Boolean) (ElapsedSeconds :type Float%20%28double-precision%29) (TriggeredSeconds :type Float%20%28double-precision%29) (InputAction :type Input%20Action%20Object%20Reference :default "/Game/Inputs/IA_Interact.IA_Interact"))
  (bind _cameracomponent (Variables|Default|GetCameraComponent))
  (bind _returnvalue (Transformation|GetWorldLocation _cameracomponent))
  ;[0.15 0.15 0.15 0.5] Interact system
  (bind _outhit (Collision|SphereTraceByChannel _returnvalue (+ _returnvalue (* (Math|Vector|GetForwardVector (Transformation|GetWorldRotation _cameracomponent)) 1.8e+02)) 1e+01 "TraceTypeQuery3" false 0 "None"))
  (if (.bBlockingHit (Collision|BreakHitResult _outhit))
    (if (Actor|ActorHasTag (.HitActor (Collision|BreakHitResult _outhit)) "Interactable")
      (if (not (and (Actor|ActorHasTag (.HitActor (Collision|BreakHitResult _outhit)) "Grabbable") (Utilities|IsValid (Variables|/Script/SPM2025.Grabber|GetGrabbedActor (Variables|Default|GetGrabber)))))
        (bind _asinteractable (Utilities|Casting|CastToInteractable (.HitActor (Collision|BreakHitResult _outhit))))
        (Class|Interactable|OnInteract _asinteractable _outhit)))
    (elif (Utilities|IsValid (Variables|/Script/SPM2025.Grabber|GetGrabbedActor (Variables|Default|GetGrabber)))
      (Class|Grabber|Release (Variables|Default|GetGrabber)))))

(event Input|EnhancedActionEvents|EnhancedInputActionIA_HoldBreath
  (params (ActionValue :type Boolean) (ElapsedSeconds :type Float%20%28double-precision%29) (TriggeredSeconds :type Float%20%28double-precision%29) (InputAction :type Input%20Action%20Object%20Reference :default "/Game/Inputs/IA_HoldBreath.IA_HoldBreath"))
  ;[0.15 0.15 0.15 0.5] Hold breath input
  (:Started
    (if (and (< (Variables|/Game/Blueprints/InGame_Widgets/WBP_HeartbeatUI.WBP_HeartbeatUI_C|GetBPM (Variables|Default|GetHeartRateUI)) 220) (not (Variables|Default|GetbIsHiding)))
      (Audio|PlaySound2D "/Game/VA_Audio/Player_Audio/HoldBreathCue.HoldBreathCue" 1.0 1.0 0.0 0 0)
      (Default|CallStartHoldBreath)
      (CallFunction|SetSpeed 0.0)
      (Variables|Default|SetTargetFOV 105.0)
      (Variables|Default|SetIsHoldingBreath true)
      (Variables|Default|SetCanRegen false)
      (Variables|Default|SetIsSprinting false)
      (Variables|/Game/Blueprints/InGame_Widgets/WBP_HoldBreathVFX.WBP_HoldBreathVFX_C|SetTargetVignette (Variables|Default|GetHoldBreathUI) 1.0)))
  (:Completed
    (if (Variables|Default|GetIsHoldingBreath)
      (Audio|PlaySound2D "/Game/VA_Audio/Player_Audio/BreathOutCue.BreathOutCue" 1.0 1.0 0.0 0 0)
      (Default|CallReleaseBreath)
      (CallFunction|ReleaseYourBreath))))

(event Input|EnhancedActionEvents|EnhancedInputActionIA_Recharge
  (params (ActionValue :type Boolean) (ElapsedSeconds :type Float%20%28double-precision%29) (TriggeredSeconds :type Float%20%28double-precision%29) (InputAction :type Input%20Action%20Object%20Reference :default "/Game/Inputs/IA_Recharge.IA_Recharge"))
  (:Started
    (CallFunction|RechargeFlashlight)))

(event EventBeginPlay
  (Variables|Default|SetDefaultSpeed (Variables|/Script/Engine.CharacterMovementComponent|GetMaxWalkSpeed (Variables|Character|GetCharacterMovement)))
  (CallFunction|StartTutorial)
  (Pawn|Components|CharacterMovement|DisableMovement (Variables|Character|GetCharacterMovement))
  (Input|SetIgnoreLookInput (Game|GetPlayerController 0) true)
  (bind _returnvalue (UserInterface|CreateWidget "/Game/Blueprints/InGame_Widgets/WBP_MainUI.WBP_MainUI_C"))
  (bind _output_get (Variables|Default|SetMainUI _returnvalue))
  (UserInterface|Viewport|AddtoViewport _output_get 0)
  (bind _returnvalue_2 (UserInterface|CreateWidget "/Game/Blueprints/InGame_Widgets/WBP_HeartbeatUI.WBP_HeartbeatUI_C"))
  (bind _output_get_2 (Variables|Default|SetHeartRateUI _returnvalue_2))
  (UserInterface|Viewport|AddtoViewport _output_get_2 0)
  (bind _returnvalue_3 (UserInterface|CreateWidget "/Game/Blueprints/InGame_Widgets/WBP_HoldBreathVFX.WBP_HoldBreathVFX_C"))
  (bind _output_get_3 (Variables|Default|SetHoldBreathUI _returnvalue_3))
  (UserInterface|Viewport|AddtoViewport _output_get_3 0)
  (bind _output_get_4 (Variables|Default|SetFOV 9e+01))
  (Variables|Default|SetTargetFOV _output_get_4)
  (EventDispatchers|BindEventtoMinigameWon (Variables|Default|GetHeartRateUI) (delegate Custom|MingameWinner))
  (Utilities|Time|SetTimerbyFunctionName 0 "CorrectFOV" 0.01 true)
  (bind _returnvalue_4 (Actor|GetActorOfClass "/Script/SPM2025.NPC_AIController"))
  (Variables|Default|SetAIController _returnvalue_4)
  (EventDispatchers|BindEventtoOnPlayerDeath (delegate Custom|OnDeathEvent))
  (EventDispatchers|BindEventtoMinigameFailed (delegate Custom|FailedMinigame)))

(event EventTick
  (params (DeltaSeconds :type Float%20%28single-precision%29))
  (CallFunction|ManageSoundandCameraShake)
  (CallFunction|UpdateStaminaBar DeltaSeconds)
  (CallFunction|CalculateandUpdateMaxStamina)
  (CallFunction|InteractPrompt))

(event EventSaveData
  (params (SaveGameInstance :type Requiem%20Save%20Game%20Object%20Reference))
  (Variables|/Script/SPM2025.RequiemSaveGame|SetPlayerSaveData SaveGameInstance (Utilities|Struct|MakePlayerSaveData (Transformation|GetActorLocation) (Transformation|GetActorRotation) (Variables|Default|GetTutorialBools) (Variables|Default|GetKeys))))

(event EventLoadData
  (params (SaveGameInstance :type Requiem%20Save%20Game%20Object%20Reference))
  (bind _playersavedata (Variables|/Script/SPM2025.RequiemSaveGame|GetPlayerSaveData SaveGameInstance))
  (Variables|Default|SetTutorialBools (.tutorialbools _playersavedata))
  (bind _output_get (Variables|Default|SetKeys (.keys _playersavedata)))
  (bind _outactors (Actor|GetAllActorsOfClass "/Game/Blueprints/KeyDoor.KeyDoor_C"))
  (for _array_element _outactors
    (if (Utilities|Array|ContainsItem _output_get (Variables|/Game/Blueprints/KeyDoor.KeyDoor_C|GetRequiredKey _array_element))
      (Default|OpenDoor _array_element)))
  (bind _outactors_2 (Actor|GetAllActorsOfClass "/Game/Blueprints/Key.Key_C"))
  (for _array_element_2 _outactors_2
    (if (Utilities|Array|ContainsItem _output_get (Variables|/Game/Blueprints/Key.Key_C|GetKeyName _array_element_2))
      (Actor|DestroyActor _array_element_2)))
  (Transformation|SetActorLocation (.position _playersavedata) false false)
  (Pawn|SetControlRotation (Pawn|GetController) (.rotation _playersavedata))
  (if (Utilities|Array|Get(acopy) (Variables|Default|GetTutorialBools))
    ;[0.15 0.15 0.15 0.5] Tutorial
    (Widget|SetVisibility (Variables|/Game/Blueprints/InGame_Widgets/WBP_MainUI.WBP_MainUI_C|GetFlashlightTutorial (Variables|Default|GetMainUI)) "Hidden")
    (Pawn|Components|CharacterMovement|SetMovementMode (Variables|Character|GetCharacterMovement) "MOVE_Walking" 0)
    (Input|SetIgnoreLookInput (Game|GetPlayerController 0) false)
    (bind _newtrack_0 (Timeline|Timeline_0 Play)
      (:Update
        (Rendering|Components|Light|SetIntensity (Variables|Default|GetPointLight) _newtrack_0)))))

(event Input|KeyboardEvents|F
  (params (Key :type Key%20Structure :default "None"))
  ;[0.15 0.15 0.15 0.5] Tutorial
  (:Pressed
    (if (not (Utilities|Array|Get(acopy) (Variables|Default|GetTutorialBools)))
      (Utilities|Array|SetArrayElem (Variables|Default|GetTutorialBools) 0 true)
      (Widget|SetVisibility (Variables|/Game/Blueprints/InGame_Widgets/WBP_MainUI.WBP_MainUI_C|GetFlashlightTutorial (Variables|Default|GetMainUI)) "Hidden")
      (Pawn|Components|CharacterMovement|SetMovementMode (Variables|Character|GetCharacterMovement) "MOVE_Walking" 0)
      (Input|SetIgnoreLookInput (Game|GetPlayerController 0) false)
      (bind _newtrack_0 (Timeline|Timeline_0 Play)
        (:Update
          (Rendering|Components|Light|SetIntensity (Variables|Default|GetPointLight) _newtrack_0))))))

(event Input|KeyboardEvents|P
  (params (Key :type Key%20Structure :default "None"))
  ;[0.15 0.15 0.15 0.5] Pause Menu
  (:Pressed
    (Game|SetGamePaused true)
    (bind _returnvalue (UserInterface|CreateWidget "/Game/Blueprints/Menu_Widgets/WBP_PauseMenu.WBP_PauseMenu_C"))
    (UserInterface|Viewport|AddtoViewport _returnvalue 0)
    (Variables|/Script/Engine.PlayerController|SetbShowMouseCursor (Game|GetPlayerController 0) true)))

(fn ConstructionScript)

(fn InteractwithHidingspot
  (params (Target :type BP%20Hiding%20Spot%20Object%20Reference)))

(fn ManageSoundandCameraShake
  (bind _returnvalue (Transformation|GetActorLocation))
  (bind _returnvalue_2 (Game|GetPlayerController 0))
  (bind _self self)
  (bind _footstepwalk (Variables|Default|GetFootstepWalk))
  (if (or (Variables|Default|GetbIsHiding) (Variables|Default|GetIsHoldingBreath))
    (Audio|Components|Audio|Stop (Variables|Default|GetFootstepWalk))
    (Audio|Components|Audio|Stop (Variables|Default|GetFootstepsSprint))
    (elif (Variables|Default|GetIsSprinting)
      (Class|AISenseHearing|ReportNoiseEvent _returnvalue 2.0 _self 1e+03 "None")
      (Game|Feedback|ClientStartCameraShake _returnvalue_2 "/Game/Blueprints/BP_SprintCameraShake.BP_SprintCameraShake_C" 1.0 "CameraLocal" "0, 0, 0")
      (if (Audio|Components|Audio|IsPlaying _footstepwalk)
        (Audio|Components|Audio|Stop _footstepwalk))
      (elif (> (Math|Vector|VectorLength (Transformation|GetVelocity)) 1.0)
        (Class|AISenseHearing|ReportNoiseEvent _returnvalue 2.0 _self 5e+02 "None")
        (Game|Feedback|ClientStartCameraShake _returnvalue_2 "/Game/Blueprints/BP_WalkCameraShake.BP_WalkCameraShake_C" 1.0 "CameraLocal" "0, 0, 0")
        (if (not (Audio|Components|Audio|IsPlaying _footstepwalk))
          (Audio|Components|Audio|Play _footstepwalk 0.0))
        (else
          (Class|AISenseHearing|ReportNoiseEvent _returnvalue 2.0 _self (+ (Math|Conversions|ToFloat(Integer) (Variables|/Game/Blueprints/InGame_Widgets/WBP_HeartbeatUI.WBP_HeartbeatUI_C|GetBPM (Variables|Default|GetHeartRateUI))) 1.8e+02) "None")
          (Game|Feedback|ClientStartCameraShake _returnvalue_2 "/Game/Blueprints/BP_IdleCameraShake.BP_IdleCameraShake_C" 1.0 "CameraLocal" "0, 0, 0")
          (if (Audio|Components|Audio|IsPlaying _footstepwalk)
            (Audio|Components|Audio|Stop _footstepwalk)))))))

(fn UpdateStaminaBar
  (params (InputPin :type Float%20%28single-precision%29))
  (bind _returnvalue (* InputPin 0.4))
  (bind _returnvalue_2 (|(Clamp(({CD1B3F10-46F3-894B-1975-A29A1DC4F7C3}-float),0.000000,{8A533D1D-454A-8B3D-052C-95965139240A})) _returnvalue))
  (if (Variables|Default|GetIsSprinting)
    (if (<= _returnvalue_2 0.0)
      (Variables|Default|SetCanRegen false)
      (Variables|Default|SetIsSprinting false)
      (Default|ChangeBPM (Variables|Default|GetHeartRateUI) (* (Variables|Default|GetDecreaseByThisMuch) -1) false)
      (Utilities|Time|SetTimerbyFunctionName 0 "StaminaCooldown" 1.5)
      (CallFunction|SetSpeed 1.0)
      (Audio|Components|Audio|Stop (Variables|Default|GetFootstepsSprint)))
    (Variables|Default|SetStamina _returnvalue_2)
    (elif (Variables|Default|GetCanRegen)
      (Variables|Default|SetStamina (|(Clamp(({CD1B3F10-46F3-894B-1975-A29A1DC4F7C3}+float),0.000000,{8A533D1D-454A-8B3D-052C-95965139240A})) (* _returnvalue (Variables|Default|GetMaxStamina)))))))

(fn CalculateandUpdateMaxStamina
  (bind _output_get (Variables|Default|SetMaxStamina (|((((0.500000-1)/(220.000000-60.000000))*BPM)+1.187500) (Math|Conversions|ToFloat(Integer) (Variables|/Game/Blueprints/InGame_Widgets/WBP_HeartbeatUI.WBP_HeartbeatUI_C|GetBPM (Variables|Default|GetHeartRateUI))))))
  (if (< _output_get (Variables|Default|GetStamina))
    (Variables|Default|SetStamina _output_get)))

(fn ExitLocker
  (Variables|Default|SetbIsHiding false)
  (Transformation|SetActorLocation (+ (Transformation|GetActorLocation) (* (Math|Vector|GetForwardVector (Transformation|GetActorRotation)) 1e+02)) false false)
  (Pawn|Components|CharacterMovement|SetMovementMode (Variables|Character|GetCharacterMovement) "MOVE_Walking" 0))

(fn RechargeFlashlight
  (if (and (not (Variables|Default|GetbIsHiding)) (Variables|Default|GetCanShake))
    (Variables|Default|SetCanShake false)
    (Default|ChangeBPM (Variables|Default|GetHeartRateUI) 25 false)
    (bind _asbp_flashlight (Utilities|Casting|CastToBP_Flashlight (Variables|Default|GetFlashlight)))
    (Variables|/Game/Blueprints/BP_Flashlight.BP_Flashlight_C|SetBattery _asbp_flashlight 1.3e+02)
    (Variables|/Script/SPM2025.Flashlight|SetbCanLight _asbp_flashlight true)
    (Class|AISenseHearing|ReportNoiseEvent (Transformation|GetActorLocation) 1e+01 _asbp_flashlight 0.0 "None")
    (Components|Animation|PlayAnimation (Variables|Default|GetArmSkeleton) "/Game/Anims/ArmAnim.ArmAnim" false)
    (Audio|SpawnSound2D "/Game/Assets/Sounds/ShakeLight.ShakeLight" 3.0 1.0 0.0 0)
    (Utilities|Time|SetTimerbyFunctionName 0 "ResetShakeCooldown" 2.5)
    (if (Utilities|IsValid (Variables|/Game/Blueprints/InGame_Widgets/WBP_MainUI.WBP_MainUI_C|GetUnitToBlink (Variables|Default|GetMainUI)))
      (Widget|SetRenderOpacity (Variables|/Game/Blueprints/InGame_Widgets/WBP_MainUI.WBP_MainUI_C|GetUnitToBlink (Variables|Default|GetMainUI)) 1.0)
      (Variables|/Game/Blueprints/InGame_Widgets/WBP_MainUI.WBP_MainUI_C|SetUnitToBlink (Variables|Default|GetMainUI) 0))))

(fn CorrectFOV
  (bind _cameracomponent (Variables|Default|GetCameraComponent))
  (if (< (Variables|Default|GetFOV) (Variables|Default|GetTargetFOV))
    (bind _output_get (Variables|Default|SetFOV (+ (Variables|Default|GetFOV) 0.05)))
    (Camera|SetFieldOfView _cameracomponent _output_get)
    (elif (> (Variables|Default|GetFOV) (Variables|Default|GetTargetFOV))
      (bind _output_get_2 (Variables|Default|SetFOV (+ (Variables|Default|GetFOV) -0.05)))
      (Camera|SetFieldOfView _cameracomponent _output_get_2))))