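; BP_Beads is an interactable beads object whose custom-depth glow turns off once it has been moved.
; BeginPlay sets HasMoved by comparing the actor's location before and after the parent's BeginPlay.
; The first interaction also sets HasMoved through a DoOnce, and every interaction passes on to the parent.
; When HasMoved is true, UpdateGlow adds a "Highlight" tag and disables custom depth on the mesh.
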(event `self.ReceiveBeginPlay`
  (`self.OnBeginPlay`)
  (`self.UpdateGlow`))

(event `self.OnInteract`
  (params (HitResult :type "HitResult Structure"))
  (`|ExecutionSequence`
    (:`then_0`
      (`/Engine/EditorBlueprintResources/StandardMacros.DoOnce` false
        (:`Completed`
          (set `self.HasMoved` true)
          (`self.UpdateGlow`))))
    (:`then_1`
      (`parent.OnInteract` HitResult))))

(fn `OnBeginPlay`
  (locals (OriginalLocation :type "Vector Structure"))
  (set `local.OriginalLocation` (`self.K2_GetActorLocation`))
  (`parent.ReceiveBeginPlay`)
  (set `self.HasMoved` (!= (`local.OriginalLocation`) (`self.K2_GetActorLocation`) :`ErrorTolerance` 1.0)))

(fn `UpdateGlow`
  (if (`self.HasMoved`)
    (`KismetArrayLibrary.Array_Add` (`self.Tags`) "Highlight")
    (`PrimitiveComponent.SetRenderCustomDepth` (`self.StaticMeshComponent`) false)))

(fn `UserConstructionScript`
  (`parent.UserConstructionScript`))