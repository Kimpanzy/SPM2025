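; BP_HidingSpot is an interactable locker the player can hide in and exit, with a state-based prompt.
; Hiding disables the flashlight and movement, then snaps player position and view to the locker mesh.
; If the boss AI pawn is within alert range, it reports noise outside, blocks exit and starts the heart-rate minigame UI.
; Exiting, when allowed, moves the player forward and restores walking and flashlight; death and minigame-failure handlers are empty.
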(event `self.ReceiveBeginPlay`
  (bind _player (`self.Player`))
  (bind _asbp_player (cast `/Game/Blueprints/BP_Player` (`GameplayStatics.GetPlayerPawn` 0)))
  (set `self.Player` _asbp_player)
  (`KismetSystemLibrary.Delay` 0.05)
  (add `PlayerCharacter.OnPlayerDeath` _player (delegate `OnPlayerDeath`))
  (add `/Game/Blueprints/BP_Player.MinigameFailed` _player (delegate `OnMinigameFailed`)))

(event `OnPlayerDeath`
  (params (Killer :type "Actor Object Reference")))

(event `OnMinigameFailed`)

(event `self.OnInteract`
  (params (HitResult :type "HitResult Structure"))
  (bind _player (`self.Player`))
  (bind _player_2 (`self.Player`))
  (bind _player_3 (`self.Player`))
  (bind _player_4 (`self.Player`))
  ; OnInteract
  (if (not (`PlayerCharacter.bIsHiding` _player_3))
    (set `PlayerCharacter.bIsHiding` true _player)
    (bind _asbp_flashlight (cast `/Game/Blueprints/BP_Flashlight` (`PlayerCharacter.Flashlight` _player)))
    (`/Game/Blueprints/BP_Flashlight.TurnOffAndDisable` _asbp_flashlight)
    (`self.SetPlayerInsideLocker`)
    ; CheckForBoss
    (if (< (`KismetMathLibrary.Vector_Distance` (`self.K2_GetActorLocation`) (`self.K2_GetActorLocation` (`Controller.K2_GetPawn` (`PlayerCharacter.AIController` (`self.Player`))))) (`self.LockerBossAlertRange`))
      (`self.ReportNoiseInfrontOfLocker`)
      (set `/Game/Blueprints/BP_Player.CanExitHidingSpot` false _player_4)
      (`/Game/Blueprints/InGame_Widgets/WBP_HeartbeatUI.StartWithTutorial` (`/Game/Blueprints/BP_Player.HeartRateUI` _player_4)))
    (elif (`/Game/Blueprints/BP_Player.CanExitHidingSpot` _player_3)
      (set `PlayerCharacter.bIsHiding` false _player_2)
      (`self.SetPlayerOutsideLocker`)
      (bind _asbp_flashlight_2 (cast `/Game/Blueprints/BP_Flashlight` (`PlayerCharacter.Flashlight` _player_2)))
      (set `Flashlight.bCanLight` true _asbp_flashlight_2))))

(event `self.ReceiveTick`
  (params (DeltaSeconds :type "Float (single-precision)"))
  ; CheckForBoss
)

(fn `GetInteractPrompt`
  (params (HitResult :type "HitResult Structure"))
  (returns (ReturnValue :type Text))
  (locals (ReturnText :type Text))
  (bind _player (`self.Player`))
  (if (not (`PlayerCharacter.bIsHiding` _player))
    (set `local.ReturnText` "Hide")
    (elif (`/Game/Blueprints/BP_Player.CanExitHidingSpot` _player)
      (set `local.ReturnText` "Exit")
      (else
        (set `local.ReturnText` ""))))
  (return (`local.ReturnText`)))

(fn `ReportNoiseInfrontOfLocker`
  (bind _returnvalue (`self.K2_GetActorRotation`))
  (`AISense_Hearing.ReportNoiseEvent` (+ (`self.K2_GetActorLocation`) (* (`KismetMathLibrary.GetRightVector` _returnvalue) 200.0) (* (`KismetMathLibrary.GetForwardVector` _returnvalue) 40.0)) 5.0 self 10000.0))

(fn `SetPlayerInsideLocker`
  (bind _staticmeshcomponent (`self.StaticMeshComponent`))
  (bind (_returnvalue_roll _returnvalue_pitch _returnvalue_yaw) (`KismetMathLibrary.BreakRotator` (`SceneComponent.K2_GetComponentRotation` _staticmeshcomponent)))
  (bind (_returnvalue_x _returnvalue_y _returnvalue_z) (`KismetMathLibrary.BreakVector` (+ (+ (* (`KismetMathLibrary.GetForwardVector` (`KismetMathLibrary.MakeRotator` _returnvalue_roll _returnvalue_pitch _returnvalue_yaw)) 42.0) (`SceneComponent.K2_GetComponentLocation` _staticmeshcomponent)) (* (`KismetMathLibrary.GetRightVector` (`KismetMathLibrary.MakeRotator` _returnvalue_roll _returnvalue_pitch _returnvalue_yaw)) -30.0))))
  (`CharacterMovementComponent.DisableMovement` (`Character.CharacterMovement` (`self.Player`)))
  (`Controller.SetControlRotation` (`GameplayStatics.GetPlayerController` 0) (`KismetMathLibrary.MakeRotator` 0.0 0.0 (+ _returnvalue_yaw 90.0)))
  (`self.K2_SetActorLocation` (`self.Player`) (`KismetMathLibrary.MakeVector` _returnvalue_x _returnvalue_y (+ _returnvalue_z 100.0)) false false))

(fn `SetPlayerOutsideLocker`
  (bind _player (`self.Player`))
  (bind _player_2 (`self.Player`))
  (`self.K2_SetActorLocation` _player (+ (`self.K2_GetActorLocation` _player_2) (* (`KismetMathLibrary.GetForwardVector` (`self.K2_GetActorRotation` _player_2)) 100.0)) false false)
  (`CharacterMovementComponent.SetMovementMode` (`Character.CharacterMovement` _player) "MOVE_Walking" 0))

(fn `UserConstructionScript`)