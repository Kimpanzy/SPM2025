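; Puzzle light ray source that casts a ray along its forward vector every game and editor tick, drawn as debug lines.
; A recursive 500-unit line trace continues from each mirror hit along the surface normal rather than a true reflection, capped by MaxBounces.
; A non-mirror hit at a new location calls RayHit on the actor's light ray trigger component through BPI_LightRayTarget.
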(event `/Game/Blueprints/BPI_EditorTick.Editor Tick`
  (`self.UpdateLightRay` (`self.K2_GetActorLocation`) (`self.GetActorForwardVector`) null true))

(event `self.ReceiveTick`
  (params (DeltaSeconds :type "Float (single-precision)"))
  (`self.UpdateLightRay` (`self.K2_GetActorLocation`) (`self.GetActorForwardVector`)))

(fn `UpdateLightRay`
  (params (SourceLocation :type "Vector Structure") (SourceDirection :type "Vector Structure") (PreviousHit :type "Actor Object Reference") (IsEditor :type Boolean))
  (bind (_outhit _returnvalue) (`KismetSystemLibrary.LineTraceSingleForObjects` SourceLocation (+ SourceLocation (* SourceDirection 500.0)) (`|MakeArray` "ObjectTypeQuery2" :!type "EObjectTypeQuery Enum") false (`|MakeArray` PreviousHit) "ForDuration" true (struct :`R` 1.0 :`A` 1.0) (struct :`G` 1.0 :`A` 1.0) 2.0))
  (if _returnvalue
    (`KismetSystemLibrary.IsObjectOfSoftClass` (`.HitActor` (`GameplayStatics.BreakHitResult` _outhit)) "/Script/SPM2025.Mirror"
      (:`True`
        (bind _result (`/Engine/EditorBlueprintResources/StandardMacros.IncrementInt` (`self.Bounces`))
          (:`  `
            (if (<= _result (`self.MaxBounces`))
              (`self.UpdateLightRay` (`.Location` (`GameplayStatics.BreakHitResult` _outhit)) (`.Normal` (`GameplayStatics.BreakHitResult` _outhit)) (`.HitActor` (`GameplayStatics.BreakHitResult` _outhit)))
              (else
                (set `self.Bounces` 0)
                (set `self.LastHit` (0.0 0.0 0.0)))))))
      (:`False`
        (if (and (!= (`.Location` (`GameplayStatics.BreakHitResult` _outhit)) (`self.LastHit`) :`ErrorTolerance` 0.001) (not IsEditor))
          (bind _asbpi_light_ray_target (cast `/Game/Blueprints/Puzzle/BPI_LightRayTarget` (`self.GetComponentByClass` (`.HitActor` (`GameplayStatics.BreakHitResult` _outhit)) "/Game/Blueprints/Puzzle/BP_LightRayTriggerComponent.BP_LightRayTriggerComponent_C")))
          (`/Game/Blueprints/Puzzle/BPI_LightRayTarget.Ray Hit` _asbpi_light_ray_target)
          (set `self.LastHit` (`.Location` (`GameplayStatics.BreakHitResult` _outhit))))))))

(fn `UserConstructionScript`
  (`AddComponent|NODE_AddChildActorComponent-0`))