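; Library puzzle actor that slides a wall aside once the player places a held book in its slot.
; On interact, it checks that the hit component's name ends in "L" and the Grabber holds a "Book"-tagged actor, then releases it at SlotL.
; It locks the book by disabling physics and stripping interaction tags, then a Timeline slides MovingWall.
; GetInteractPrompt shows placement or missing-book text; a generic slot swap helper is never called here.
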(event `self.ReceiveBeginPlay`
  (bind _asbp_player (cast `/Game/Blueprints/BP_Player` (`GameplayStatics.GetPlayerPawn` 0)))
  (set `self.Grabber` (`/Game/Blueprints/BP_Player.Grabber` _asbp_player)))

(event `self.ReceiveActorBeginOverlap`
  (params (OtherActor :type "Actor Object Reference")))

(event `self.OnInteract`
  (params (HitResult :type "HitResult Structure"))
  (bind _returnvalue (`KismetSystemLibrary.GetDisplayName` (`.HitComponent` (`GameplayStatics.BreakHitResult` HitResult))))
  (bind _grabbedactor (`Grabber.GrabbedActor` (`self.Grabber`)))
  (bind _returnvalue_2 (`KismetStringLibrary.Len` _returnvalue))
  (if (`KismetSystemLibrary.IsValid` _grabbedactor)
    (if (and (`KismetStringLibrary.EqualEqual_StrStr` (`KismetStringLibrary.GetSubstring` _returnvalue (- _returnvalue_2 1) _returnvalue_2) "L") (`self.ActorHasTag` (`Grabber.GrabbedActor` (`self.Grabber`)) "Book"))
      (bind _asbp_artifact (cast `/Game/Blueprints/BP_Artifact` _grabbedactor))
      (`PrimitiveComponent.SetSimulatePhysics` (`StaticMeshActor.StaticMeshComponent` _asbp_artifact) false)
      (`Grabber.ReleaseAtPos` (`self.Grabber`) (+ (`SceneComponent.K2_GetComponentLocation` (`self.SlotL`)) (0.0 -10.0 -10.0)) (struct :`Yaw` 90.0 :`Roll` 45.0) true)
      (set `self.IsPlaced` true)
      (bind _tags (`Actor.Tags` _asbp_artifact))
      (`KismetArrayLibrary.Array_RemoveItem` _tags "Interactable")
      (`KismetArrayLibrary.Array_RemoveItem` _tags "Grabbable")
      (`KismetArrayLibrary.Array_RemoveItem` _tags "Highlight")
      (bind (_direction _height) (`Timeline|Timeline`)
        (:`Update`
          (`SceneComponent.K2_SetRelativeLocation` (`self.MovingWall`) (`KismetMathLibrary.MakeVector` (`KismetMathLibrary.Lerp` -350.0 -650.0 _height) -73.0) false false))))))

(fn `GetInteractPrompt`
  (params (HitResult :type "HitResult Structure"))
  (returns (ReturnValue :type Text))
  (bind _returnvalue (`KismetSystemLibrary.GetDisplayName` (`.HitComponent` (`GameplayStatics.BreakHitResult` HitResult))))
  (bind _grabbedactor (`Grabber.GrabbedActor` (`self.Grabber`)))
  (bind _returnvalue_2 (`KismetStringLibrary.Len` _returnvalue))
  (if (`KismetStringLibrary.EqualEqual_StrStr` (`KismetStringLibrary.GetSubstring` _returnvalue (- _returnvalue_2 1) _returnvalue_2) "L")
    (if (`KismetSystemLibrary.IsValid` _grabbedactor)
      (if (`self.ActorHasTag` _grabbedactor "Book")
        (return "Place")
        (else
          _)))
    (if (`self.IsPlaced`)
      (return "")
      (else
        (return "Missing book")))
    (else
      (return ""))))

(fn `NewFunction`
  (params (SlotObject :type "Actor Object Reference") (Slot :type "BoxComponent Object Reference"))
  (returns (SlotObjectReturn :type "Actor Object Reference") (ReturnObject :type "Actor Object Reference"))
  (locals (ReturnLObject :type "Actor Object Reference"))
  (bind _grabber (`self.Grabber`))
  (set `local.ReturnLObject` SlotObject)
  (if (`KismetSystemLibrary.IsValid` (`local.ReturnLObject`))
    (`Grabber.Grab` :`self` (`self.Grabber`) :`HitActor` (stale _output_get))
    (set `local.ReturnLObject` null)
    (else
      (bind _output_get (set `local.ReturnLObject` (`Grabber.GrabbedActor` _grabber)))
      (`Grabber.ReleaseAtPos` :`self` _grabber :`Location` (+ (`SceneComponent.K2_GetComponentLocation` Slot) (0.0 0.0 0.0)))))
  (return (`local.ReturnLObject`) null))

(fn `UserConstructionScript`)