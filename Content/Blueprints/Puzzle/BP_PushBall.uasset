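; BP_PushBall is a pushable puzzle ball that plays a rolling sound while moving and keeps its position across saves.
; Tick starts the BallRoll sound when velocity passes a small threshold and stops it otherwise.
; On BeginPlay it requests a load from the RequiemGameInstance; its save and load events store and restore location and rotation in the PushableBalls map, keyed by ID.
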(event `self.ReceiveBeginPlay`
  (bind _asrequiem_game_instance (cast `RequiemGameInstance` (`GameplayStatics.GetGameInstance`)))
  (`Persistence.RequestLoad` _asrequiem_game_instance self))

(event `self.ReceiveTick`
  (params (DeltaSeconds :type "Float (single-precision)"))
  (if (> (`KismetMathLibrary.VSize` (`self.GetVelocity`)) 5.0)
    (if (not (`AudioComponent.IsPlaying` (`self.BallRoll`)))
      (`AudioComponent.Play` (`self.BallRoll`) 0.0))
    (else
      (`AudioComponent.Stop` (`self.BallRoll`)))))

(event `self.SaveData`
  (params (SaveGameInstance :type "RequiemSaveGame Object Reference"))
  (`BlueprintMapLibrary.Map_Add` (`RequiemSaveGame.PushableBalls` SaveGameInstance) (`self.ID`) (make `PushableBallSaveData` (`self.K2_GetActorLocation`) (`self.K2_GetActorRotation`))))

(event `self.LoadData`
  (params (SaveGameInstance :type "RequiemSaveGame Object Reference"))
  (bind (_value _returnvalue) (`BlueprintMapLibrary.Map_Find` (`RequiemSaveGame.PushableBalls` SaveGameInstance) (`self.ID`)))
  (if _returnvalue
    (`self.K2_SetActorLocationAndRotation` (break `PushableBallSaveData` _value) (`.Rotation` (break `PushableBallSaveData` _value)))))

(fn `UserConstructionScript`)