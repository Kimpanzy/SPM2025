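; Library puzzle actor where the player arranges five books by color tag to slide open a wall.
; Interaction takes the slot index from the last character of the hit component's name, then grabs or places a book through the player's Grabber, toggling its trace collision.
; Each placement checks the order; solving it locks the books, plays a scraping sound and moves the wall on a Timeline.
; GetInteractPrompt returns text matching slot and hand state.
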(event `self.ReceiveBeginPlay`
  (bind _boxcolliders (`self.BoxColliders`))
  (`KismetArrayLibrary.Array_Add` _boxcolliders (`self.0`))
  (`KismetArrayLibrary.Array_Add` _boxcolliders (`self.1`))
  (`KismetArrayLibrary.Array_Add` _boxcolliders (`self.2`))
  (`KismetArrayLibrary.Array_Add` _boxcolliders (`self.3`))
  (`KismetArrayLibrary.Array_Add` _boxcolliders (`self.4`))
  (bind _asbp_player (cast `/Game/Blueprints/BP_Player` (`GameplayStatics.GetPlayerCharacter` 0)))
  (set `self.Grabber` (`/Game/Blueprints/BP_Player.Grabber` _asbp_player)))

(event `self.OnInteract`
  (params (HitResult :type "HitResult Structure"))
  (bind _grabber (`self.Grabber`))
  (bind _returnvalue (`KismetSystemLibrary.GetDisplayName` (`.HitComponent` (`GameplayStatics.BreakHitResult` HitResult))))
  (bind _returnvalue_2 (`KismetStringLibrary.Len` _returnvalue))
  (bind _returnvalue_3 (`KismetStringLibrary.Conv_StringToInt` (`KismetStringLibrary.GetSubstring` _returnvalue (- _returnvalue_2 1) _returnvalue_2)))
  (bind _output (`|GetArrayItem` (`self.Books`) _returnvalue_3))
  (bind _output_2 (`|GetArrayItem` (`self.BoxColliders`) _returnvalue_3))
  (bind _output_3 (`|GetArrayItem` (`self.Books`) _returnvalue_3))
  (if (`KismetSystemLibrary.IsValid` _output)
    (if (not (`self.Won`))
      (if (not (`KismetSystemLibrary.IsValid` (`Grabber.GrabbedActor` (`self.Grabber`))))
        (`Grabber.Grab` (`self.Grabber`) _output_3 (0.0 0.0 20.0) (struct :`Roll` 90.0) true)
        (`KismetArrayLibrary.Array_Set` (`self.Books`) _returnvalue_3 null true)
        (bind _asstatic_mesh_actor (cast `StaticMeshActor` _output_3))
        (`PrimitiveComponent.SetCollisionResponseToChannel` (`StaticMeshActor.StaticMeshComponent` _asstatic_mesh_actor) "ECC_GameTraceChannel1" "ECR_Block")))
    (else
      (`KismetArrayLibrary.Array_Set` (`self.Books`) _returnvalue_3 (`Grabber.GrabbedActor` _grabber) true)
      (`Grabber.ReleaseAtPos` _grabber (+ (`SceneComponent.K2_GetComponentLocation` _output_2) (* (`SceneComponent.GetRightVector` _output_2) 0.5) (* (`SceneComponent.GetForwardVector` _output_2) -4.0) (* (`SceneComponent.GetUpVector` _output_2) -0.5)) (struct :`Roll` 90.0) true)
      (bind _asstatic_mesh_actor_2 (cast `StaticMeshActor` _output))
      (`PrimitiveComponent.SetCollisionResponseToChannel` (`StaticMeshActor.StaticMeshComponent` _asstatic_mesh_actor_2) "ECC_GameTraceChannel1" "ECR_Ignore")
      (`self.CheckForSolution`)
      (if (`self.Won`)
        (`GameplayStatics.PlaySoundAtLocation` "/Game/Assets/Sounds/stoneScraping.stoneScraping" (`SceneComponent.K2_GetComponentLocation` (`self.MovingWall`)) (struct) 0.8 1.0 0.0 "/Game/Assets/Sounds/ATT_BossWalking.ATT_BossWalking" null null null)
        (`KismetSystemLibrary.Delay` 1.5)
        (bind (_direction _height) (`Timeline|Timeline`)
          (:`Update`
            (`SceneComponent.K2_SetRelativeLocation` (`self.MovingWall`) (`KismetMathLibrary.MakeVector` (`KismetMathLibrary.Lerp` -613.0 -913.0 _height) -9.228513) false false)))))))

(fn `CheckForSolution`
  (if (and (`KismetSystemLibrary.IsValid` (`|GetArrayItem` (`self.Books`))) (`KismetSystemLibrary.IsValid` (`|GetArrayItem` (`self.Books`) 1)) (`KismetSystemLibrary.IsValid` (`|GetArrayItem` (`self.Books`) 2)) (`KismetSystemLibrary.IsValid` (`|GetArrayItem` (`self.Books`) 3)) (`KismetSystemLibrary.IsValid` (`|GetArrayItem` (`self.Books`) 4)) true)
    (if (and (`self.ActorHasTag` (`|GetArrayItem` (`self.Books`)) "Blue") (`self.ActorHasTag` (`|GetArrayItem` (`self.Books`) 1) "Purple") (`self.ActorHasTag` (`|GetArrayItem` (`self.Books`) 2) "Yellow") (`self.ActorHasTag` (`|GetArrayItem` (`self.Books`) 3) "Green") (`self.ActorHasTag` (`|GetArrayItem` (`self.Books`) 4) "Red") true)
      (set `self.Won` true))))

(fn `GetInteractPrompt`
  (params (HitResult :type "HitResult Structure"))
  (returns (ReturnValue :type Text))
  (bind _returnvalue (`KismetSystemLibrary.GetDisplayName` (`.HitComponent` (`GameplayStatics.BreakHitResult` HitResult))))
  (bind _returnvalue_2 (`KismetStringLibrary.Len` _returnvalue))
  (if (`KismetSystemLibrary.IsValid` (`|GetArrayItem` (`self.Books`) (`KismetStringLibrary.Conv_StringToInt` (`KismetStringLibrary.GetSubstring` _returnvalue (- _returnvalue_2 1) _returnvalue_2))))
    (if (not (`self.Won`))
      (if (`KismetSystemLibrary.IsValid` (`Grabber.GrabbedActor` (`self.Grabber`)))
        (return "Already Holding Item")
        (else
          (return "Grab")))
      (else
        (return "")))
    (elif (`KismetSystemLibrary.IsValid` (`Grabber.GrabbedActor` (`self.Grabber`)))
      (return "Place")
      (else
        (return "Missing book")))))

(fn `UserConstructionScript`)