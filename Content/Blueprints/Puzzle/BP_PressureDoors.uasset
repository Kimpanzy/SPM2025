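; BP_PressureDoors is a puzzle double door that the player opens by stepping on a pressure plate and later closes through a trigger.
; The plate overlap destroys the plate and plays a timeline that swings both door meshes in opposite directions by lerped rotation.
; A separate close trigger destroys itself and reverses the timeline.
; The timeline's Finished event requests a save through RequiemGameInstance.
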(event `self.Second_Plate.OnComponentBeginOverlap`
  (params (OverlappedComponent :type "PrimitiveComponent Object Reference") (OtherActor :type "Actor Object Reference") (OtherComp :type "PrimitiveComponent Object Reference") (OtherBodyIndex :type Integer) (bFromSweep :type Boolean) (SweepResult :type "HitResult Structure (by ref)"))
  (cast `/Game/Blueprints/BP_Player` OtherActor)
  (`ActorComponent.K2_DestroyComponent` (`self.Second_Plate`))
  (bind (_direction _height) (`Timeline|PlayerPressure` :!label _label)
    (:`Update`
      (`|ExecutionSequence`
        (:`then_0`
          (`SceneComponent.K2_SetRelativeRotation` (`self.SM_Door1`) (`KismetMathLibrary.RLerp` (struct :`Yaw` -180.0) (struct :`Yaw` -260.0) _height) false false))
        (:`then_1`
          (`SceneComponent.K2_SetRelativeRotation` (`self.SM_Door`) (`KismetMathLibrary.RLerp` (struct :`Yaw` -180.0) (struct :`Yaw` -100.0) _height) false false))))
    (:`Finished`
      (bind _asrequiem_game_instance (cast `RequiemGameInstance` (`GameplayStatics.GetGameInstance`)))
      (`Persistence.RequestSave` _asrequiem_game_instance true))))

(event `self.CloseTrigger.OnComponentBeginOverlap`
  (params (OverlappedComponent :type "PrimitiveComponent Object Reference") (OtherActor :type "Actor Object Reference") (OtherComp :type "PrimitiveComponent Object Reference") (OtherBodyIndex :type Integer) (bFromSweep :type Boolean) (SweepResult :type "HitResult Structure (by ref)"))
  (cast `/Game/Blueprints/BP_Player` OtherActor)
  (`ActorComponent.K2_DestroyComponent` (`self.CloseTrigger`))
  (goto _label :!via `ReverseFromEnd`))

(fn `UserConstructionScript`)