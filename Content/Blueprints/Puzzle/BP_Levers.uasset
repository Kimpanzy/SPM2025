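; BP_Levers is an interactable puzzle lever that toggles between up and down, showing a "Pull" prompt.
; OnInteract ignores input while the lever is moving, then picks one of two timelines based on IsDown.
; Each timeline interpolates the Lever0 component's relative rotation between two fixed angles, then flips IsDown and clears the moving lock.
; It only tracks its own state and triggers nothing else.
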(event `self.OnInteract`
  (params (HitResult :type "HitResult Structure"))
  (if (not (`self.IsMoving`))
    (set `self.IsMoving` true)
    (bind _output_get (set `self.Lever_0` (`self.Lever_0`)))
    (if (`self.IsDown`)
      (bind (_direction _height) (`Timeline|Timeline_0` :!via `PlayFromStart`)
        (:`Update`
          (`SceneComponent.K2_SetRelativeRotation` _output_get (`KismetMathLibrary.RLerp` (struct :`Roll` 135.0) (struct :`Roll` 45.0) _height) false false))
        (:`Finished`
          (set `self.IsDown` false)
          (set `self.IsMoving` false)))
      (else
        (bind (_direction_2 _height_2) (`Timeline|Timeline` :!via `PlayFromStart`)
          (:`Update`
            (`SceneComponent.K2_SetRelativeRotation` _output_get (`KismetMathLibrary.RLerp` (struct :`Roll` 45.0) (struct :`Roll` 135.0) _height_2) false false))
          (:`Finished`
            (set `self.IsDown` true)
            (set `self.IsMoving` false)))))))

(fn `GetInteractPrompt`
  (params (HitResult :type "HitResult Structure"))
  (returns (ReturnValue :type Text))
  (return "Pull"))

(fn `UserConstructionScript`)