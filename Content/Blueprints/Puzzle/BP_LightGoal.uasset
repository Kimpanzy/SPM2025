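; BP_LightGoal is the target of a light-ray puzzle, which completes when a ray hit reaches it under the right condition.
; OnRayHit proceeds only if the puzzle is not yet won and the PrayerBead is away from a hardcoded world position.
; It then shifts the goal down along its mesh's up vector, latches the Won flag and prints a completion message.
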(event `self.ReceiveBeginPlay`)

(event `self.OnRayHit`
  (bind _staticmeshcomponent (`self.StaticMeshComponent`))
  (if (not (`self.Won`))
    (if (not (== (`self.K2_GetActorLocation` (`self.PrayerBead`)) (-1950.0 2630.0 0.0) :`ErrorTolerance` 1.0))
      (`self.K2_SetActorLocation` (+ (`SceneComponent.K2_GetComponentLocation` _staticmeshcomponent) (* (`SceneComponent.GetUpVector` _staticmeshcomponent) -40.0)))
      (set `self.Won` true)
      (`KismetSystemLibrary.PrintString` "Puzzle Complete!"))))

(fn `UserConstructionScript`)