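; BP_LibraryBook is a book the player can pick up, showing its name as the interact prompt.
; Interacting passes it to the player's Grabber component with fixed location and rotation offsets.
; It requests a load from the Requiem game instance on BeginPlay, saving and restoring its transform in the save game's Artifacts map.
; The map key is a GUID that the construction script regenerates on every run.
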(event `self.ReceiveBeginPlay`
  (bind _asrequiem_game_instance (cast `RequiemGameInstance` (`GameplayStatics.GetGameInstance`))
    (:`then`
      (`Persistence.RequestLoad` _asrequiem_game_instance self))
    (:`CastFailed`
      _))
  (bind _asbp_player (cast `/Game/Blueprints/BP_Player` (`GameplayStatics.GetPlayerCharacter` 0)))
  (set `self.As BP Player` _asbp_player))

(event `self.OnInteract`
  (params (HitResult :type "HitResult Structure"))
  (`Grabber.Grab` (`/Game/Blueprints/BP_Player.Grabber` (`self.As BP Player`)) self (0.0 0.0 20.0) (struct :`Roll` 90.0) false))

(event `self.SaveData`
  (params (SaveGameInstance :type "RequiemSaveGame Object Reference"))
  (`BlueprintMapLibrary.Map_Add` (`RequiemSaveGame.Artifacts` SaveGameInstance) (`self.ID`) (make `ArtifactSaveData` (`self.K2_GetActorLocation`) (`self.K2_GetActorRotation`))))

(event `self.LoadData`
  (params (SaveGameInstance :type "RequiemSaveGame Object Reference"))
  (bind (_value _returnvalue) (`BlueprintMapLibrary.Map_Find` (`RequiemSaveGame.Artifacts` SaveGameInstance) (`self.ID`)))
  (if _returnvalue
    (`self.K2_SetActorLocationAndRotation` (break `ArtifactSaveData` _value) (`.Rotation` (break `ArtifactSaveData` _value)) false true)))

(fn `GetInteractPrompt`
  (params (HitResult :type "HitResult Structure"))
  (returns (ReturnValue :type Text))
  (return (`self.Name`)))

(fn `UserConstructionScript`
  (set `self.ID` (`KismetGuidLibrary.NewGuid`)))