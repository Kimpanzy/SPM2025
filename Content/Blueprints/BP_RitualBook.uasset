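; Interactable ritual book whose skeletal mesh pages the player flips forward or back by interacting with components tagged right or left, with matching prompts.
; Flips play each page's animation forward or reversed with a sound, guarded by an index range and timer-reset lock.
; Forward flips queue the previously turned page, which Tick lowers after a countdown.
; Backward flips raise that page again after a short delay.
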(event `self.ReceiveBeginPlay`
  (set `self.Pages` (`self.K2_GetComponentsByClass` "/Script/Engine.SkeletalMeshComponent")))

(event `self.ReceiveTick`
  (params (DeltaSeconds :type "Float (single-precision)"))
  (for (_array_element _array_index) (`self.BookRepositonQueue`)
    (bind (_booktorepos _timetorepos) (break `/Game/BookRepositonQueue` _array_element))
    (bind _returnvalue (- _timetorepos DeltaSeconds))
    (bind _structout (setmembers `/Game/BookRepositonQueue` :`StructRef` _array_element :`TimeToRepos` _returnvalue))
    (`KismetArrayLibrary.Array_Set` (`self.BookRepositonQueue`) _array_index _structout)
    (if (<= _returnvalue 0.0)
      (`SceneComponent.K2_AddLocalOffset` _booktorepos (0.0 0.0 -0.3) false false)
      (`KismetArrayLibrary.Array_Remove` (`self.BookRepositonQueue`) _array_index))))

(event `self.OnInteract`
  (params (HitResult :type "HitResult Structure"))
  (bind (_bblockinghit _binitialoverlap _time _distance _location _impactpoint _normal _impactnormal _physmat _hitactor _hitcomponent) (`GameplayStatics.BreakHitResult` HitResult))
  (bind _returnvalue (`self.K2_GetActorLocation`))
  (bind _output (`|GetArrayItem` (`self.Pages`) (`self.CurrentIndex`)))
  (bind _output_2 (`|GetArrayItem` (`self.Pages`) (- (`self.CurrentIndex`) 1)))
  (if (`ActorComponent.ComponentHasTag` _hitcomponent "RitualRight")
    (if (and (< (`self.CurrentIndex`) 3) (not (`self.IsFlipping`)))
      (`GameplayStatics.SpawnSoundAtLocation` "/Game/GameAudio/Foleys_SFX/page.page" _returnvalue (struct) 1.0 1.0 0.0 null null)
      (set `self.IsFlipping` true)
      (`KismetSystemLibrary.K2_SetTimer` null "ResetIsFlipping" 0.31)
      (`SkeletalMeshComponent.SetPlayRate` _output 1.0)
      (`SkeletalMeshComponent.Play` _output false)
      (set `self.CurrentIndex` (+ (`self.CurrentIndex`) 1))
      (if (> (- (`self.CurrentIndex`) 1) 0)
        (`KismetArrayLibrary.Array_Add` (`self.BookRepositonQueue`) (make `/Game/BookRepositonQueue` (`|GetArrayItem` (`self.Pages`) (- (`self.CurrentIndex`) 2)) 1.75))))
    (elif (`ActorComponent.ComponentHasTag` _hitcomponent "RitualLeft")
      (if (and (> (`self.CurrentIndex`) 0) (not (`self.IsFlipping`)))
        (`GameplayStatics.SpawnSoundAtLocation` "/Game/GameAudio/Foleys_SFX/page.page" _returnvalue (struct) 1.0 1.0 0.0 null null)
        (set `self.IsFlipping` true)
        (`KismetSystemLibrary.K2_SetTimer` null "ResetIsFlipping" 0.31)
        (`SkeletalMeshComponent.SetPlayRate` _output_2 -1.0)
        (`SkeletalMeshComponent.Play` _output_2 false)
        (`KismetSystemLibrary.Delay` 0.3)
        (if (> (`self.CurrentIndex`) 1)
          (`SceneComponent.K2_AddLocalOffset` (`|GetArrayItem` (`self.Pages`) (- (`self.CurrentIndex`) 2)) (0.0 0.0 0.3) false false))
        (set `self.CurrentIndex` (- (`self.CurrentIndex`) 1))))))

(event `ResetIsFlipping`
  (set `self.IsFlipping` false))

(fn `GetInteractPrompt`
  (params (HitResult :type "HitResult Structure"))
  (returns (ReturnValue :type Text))
  (locals (ReturnText :type Text))
  (bind (_bblockinghit _binitialoverlap _time _distance _location _impactpoint _normal _impactnormal _physmat _hitactor _hitcomponent) (`GameplayStatics.BreakHitResult` HitResult))
  (if (`ActorComponent.ComponentHasTag` _hitcomponent "RitualRight")
    (set `local.ReturnText` "Flip Right")
    (elif (`ActorComponent.ComponentHasTag` _hitcomponent "RitualLeft")
      (set `local.ReturnText` "Flip Left")
      (else
        (set `local.ReturnText` ""))))
  (return (`local.ReturnText`)))

(fn `UserConstructionScript`)