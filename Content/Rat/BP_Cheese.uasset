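; BP_Cheese is an interactable cheese prop that the player can grab.
; It caches the player character as BP_Player on BeginPlay, and on interact hands itself to that player's Grabber with a fixed location and rotation offset.
; The IsGrabbable flag gates both the grab and the "Grab Cheese" prompt, which is empty otherwise.
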(event `self.ReceiveBeginPlay`
  (bind _asbp_player (cast `/Game/Blueprints/BP_Player` (`GameplayStatics.GetPlayerCharacter` 0)))
  (set `self.As BP Player` _asbp_player))

(event `self.OnInteract`
  (params (HitResult :type "HitResult Structure"))
  (if (`self.IsGrabbable`)
    (`Grabber.Grab` (`/Game/Blueprints/BP_Player.Grabber` (`self.As BP Player`)) self (20.0 0.0 0.0) (struct :`Pitch` 180.0 :`Roll` 180.0) false)))

(fn `GetInteractPrompt`
  (params (HitResult :type "HitResult Structure"))
  (returns (ReturnValue :type Text))
  (if (`self.IsGrabbable`)
    (return "Grab Cheese")
    (else
      (return ""))))

(fn `UserConstructionScript`)