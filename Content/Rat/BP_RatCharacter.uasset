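; BP_RatCharacter is an AI-controlled rat that the player can pick up while it is not caged.
; The IsCaged blackboard key gates both the "Pickup Rat" prompt and the interaction.
; Interacting attaches the rat through the cached player's Grabber with a fixed offset and rotation, then marks the cheese referenced by its RatAIController as grabbable.
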(event `self.ReceiveBeginPlay`
  (bind _asbp_player (cast `/Game/Blueprints/BP_Player` (`GameplayStatics.GetPlayerCharacter` 0)))
  (set `self.As BP Player` _asbp_player))

(event `self.OnInteract`
  (params (HitResult :type "HitResult Structure"))
  (if (not (`BlackboardComponent.GetValueAsBool` (`AIBlueprintHelperLibrary.GetBlackboard` (`AIBlueprintHelperLibrary.GetAIController` self)) "IsCaged"))
    (`Grabber.Grab` (`/Game/Blueprints/BP_Player.Grabber` (`self.As BP Player`)) self (-10.0 0.0 50.0) (struct :`Pitch` 90.0))
    (bind _asrat_aicontroller (cast `RatAIController` (`AIBlueprintHelperLibrary.GetAIController` self)))
    (bind _asbp_cheese (cast `/Game/Rat/BP_Cheese` (`RatAIController.Cheese` _asrat_aicontroller)))
    (set `/Game/Rat/BP_Cheese.IsGrabbable` true _asbp_cheese)))

(fn `GetInteractPrompt`
  (params (HitResult :type "HitResult Structure"))
  (returns (ReturnValue :type Text))
  (if (not (`BlackboardComponent.GetValueAsBool` (`AIBlueprintHelperLibrary.GetBlackboard` (`AIBlueprintHelperLibrary.GetAIController` self)) "IsCaged"))
    (return "Pickup Rat")
    (else
      (return ""))))

(fn `UserConstructionScript`)