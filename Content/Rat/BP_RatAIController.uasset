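; AI controller for the rat that runs its behavior tree and plays occasional squeaks.
; On BeginPlay it seeds the blackboard with the rat's caged state, first target and the level's cheese actor.
; It binds to the player's Grabber events to track whether cheese is held, clearing the flag on any drop.
; After an initial delay, a self-rescheduling timer plays pitch-varied squeals at random intervals.
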(event `self.ReceiveBeginPlay`
  (bind _returnvalue (`AIBlueprintHelperLibrary.GetBlackboard` null))
  (bind _asbp_player (cast `/Game/Blueprints/BP_Player` (`GameplayStatics.GetPlayerPawn` 0)))
  (bind _grabber (`/Game/Blueprints/BP_Player.Grabber` _asbp_player))
  (add `Grabber.ItemGrabbed` _grabber (delegate `IsItCheese?????`))
  (add `Grabber.ItemDropped` _grabber (delegate `CheeseDropped`))
  (bind _returnvalue_2 (`GameplayStatics.GetActorOfClass` "/Game/Rat/BP_Cheese.BP_Cheese_C"))
  (bind _output_get (set `self.Cheese` _returnvalue_2))
  (`self.RunBehaviorTree` "/Game/Rat/BT_Rat.BT_Rat")
  (bind _asbp_rat_character (cast `/Game/Rat/BP_RatCharacter` (`self.K2_GetPawn`)))
  (`BlackboardComponent.SetValueAsBool` (`AIBlueprintHelperLibrary.GetBlackboard` null) "IsCaged" (`/Game/Rat/BP_RatCharacter.IsCaged` _asbp_rat_character))
  (`BlackboardComponent.SetValueAsVector` _returnvalue "CurrentTarget" (`|GetArrayItem` (`self.Targets`)))
  (`BlackboardComponent.SetValueAsObject` _returnvalue "CheeseActor" _output_get)
  (`KismetSystemLibrary.Delay` 6.0)
  (`self.PlaySoundRandomly`))

(event `IsItCheese?????`
  (params (GrabbedItem :type "Actor Object Reference"))
  (if (`self.ActorHasTag` GrabbedItem "Cheese")
    (set `self.bPlayerIsHoldingCheese` true)))

(event `CheeseDropped`
  (params (DroppedItem :type "Actor Object Reference"))
  (set `self.bPlayerIsHoldingCheese` false))

(event `PlaySoundRandomly`
  (`GameplayStatics.PlaySoundAtLocation` "/Game/Assets/Sounds/rat_Cue.rat_Cue" (`self.K2_GetActorLocation` (`self.K2_GetPawn`)) (struct) 0.05 (`KismetMathLibrary.RandomFloatInRange` 0.9 1.1) 0.0 "/Game/Assets/Sounds/ATT_RatSqueal.ATT_RatSqueal" null null null)
  (`KismetSystemLibrary.K2_SetTimer` null "PlaySoundRandomly" (`KismetMathLibrary.RandomFloatInRange` 5.0 15.0)))

(fn `UserConstructionScript`)