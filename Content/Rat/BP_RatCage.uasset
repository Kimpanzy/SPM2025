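; BP_RatCage is an interactable cage where the player deposits a rat they are carrying.
; Interacting while the player's Grabber holds a "Rat"-tagged actor sets IsCaged on that rat's AI blackboard.
; After a short delay, the Grabber releases it just in front of the cage origin and RatIsInCage is set.
; The interact prompt reads "Place" when a rat is held, otherwise "Missing Rat".
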(event `self.ReceiveBeginPlay`
  (bind _asbp_player (cast `/Game/Blueprints/BP_Player` (`GameplayStatics.GetPlayerCharacter` 0)))
  (set `self.As BP Player` _asbp_player))

(event `self.OnInteract`
  (params (HitResult :type "HitResult Structure"))
  (bind _grabber (`/Game/Blueprints/BP_Player.Grabber` (`self.As BP Player`)))
  (bind _grabbedactor (`Grabber.GrabbedActor` (`/Game/Blueprints/BP_Player.Grabber` (`self.As BP Player`))))
  (if (`KismetSystemLibrary.IsValid` _grabbedactor)
    (if (`self.ActorHasTag` _grabbedactor "Rat")
      (bind _asbp_rat_character (cast `/Game/Rat/BP_RatCharacter` (`Grabber.GrabbedActor` _grabber)))
      (`BlackboardComponent.SetValueAsBool` (`AIBlueprintHelperLibrary.GetBlackboard` (`AIBlueprintHelperLibrary.GetAIController` _asbp_rat_character)) "IsCaged" true)
      (`KismetSystemLibrary.Delay` 0.2)
      (`Grabber.ReleaseAtPos` :`self` _grabber :`Location` (+ (`self.K2_GetActorLocation`) (* (`KismetMathLibrary.GetForwardVector` (`self.K2_GetActorRotation`)) 1.0)))
      (set `self.RatIsInCage` true))))

(fn `GetInteractPrompt`
  (params (HitResult :type "HitResult Structure"))
  (returns (ReturnValue :type Text))
  (bind _grabbedactor (`Grabber.GrabbedActor` (`/Game/Blueprints/BP_Player.Grabber` (`self.As BP Player`))))
  (if (`KismetSystemLibrary.IsValid` _grabbedactor)
    (if (`self.ActorHasTag` _grabbedactor "Rat")
      (return "Place")
      (else
        _)))
  (return "Missing Rat"))

(fn `UserConstructionScript`)