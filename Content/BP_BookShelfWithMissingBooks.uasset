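; Interactable bookshelf with five slots where the player takes out or places books, prompting "Missing book".
; BeginPlay collects the slot box colliders and caches the player's Grabber.
; OnInteract reads the slot index from the last character of the hit component's name.
; An occupied slot hands its book to the Grabber and clears; an empty one stores the grabbed actor and releases it at a collider-relative position with physics disabled.
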(event `self.ReceiveBeginPlay`
  (bind _boxcolliders (`self.BoxColliders`))
  (`KismetArrayLibrary.Array_Add` _boxcolliders (`self.0`))
  (`KismetArrayLibrary.Array_Add` _boxcolliders (`self.1`))
  (`KismetArrayLibrary.Array_Add` _boxcolliders (`self.2`))
  (`KismetArrayLibrary.Array_Add` _boxcolliders (`self.3`))
  (`KismetArrayLibrary.Array_Add` _boxcolliders (`self.4`))
  (bind _asbp_player (cast `/Game/Blueprints/BP_Player` (`GameplayStatics.GetPlayerCharacter` 0)))
  (set `self.Grabber` (`/Game/Blueprints/BP_Player.Grabber` _asbp_player)))

(event `self.OnInteract`
  (params (HitResult :type "HitResult Structure"))
  (bind _grabber (`self.Grabber`))
  (bind _returnvalue (`KismetSystemLibrary.GetDisplayName` (`.HitComponent` (`GameplayStatics.BreakHitResult` HitResult))))
  (bind _returnvalue_2 (`KismetStringLibrary.Len` _returnvalue))
  (bind _returnvalue_3 (`KismetStringLibrary.Conv_StringToInt` (`KismetStringLibrary.GetSubstring` _returnvalue (- _returnvalue_2 1) _returnvalue_2)))
  (bind _output (`|GetArrayItem` (`self.BoxColliders`) _returnvalue_3))
  (if (`KismetSystemLibrary.IsValid` (`|GetArrayItem` (`self.Books`) _returnvalue_3))
    (`Grabber.Grab` :`self` (`self.Grabber`) :`HitActor` (`|GetArrayItem` (`self.Books`) _returnvalue_3))
    (`KismetArrayLibrary.Array_Set` (`self.Books`) _returnvalue_3 null true)
    (else
      (`KismetArrayLibrary.Array_Set` (`self.Books`) _returnvalue_3 (`Grabber.GrabbedActor` _grabber) true)
      (`Grabber.ReleaseAtPos` _grabber (+ (`SceneComponent.K2_GetComponentLocation` _output) (* (`SceneComponent.GetRightVector` _output) -3.0) (* (`SceneComponent.GetForwardVector` _output) -4.0) (* (`SceneComponent.GetUpVector` _output) 9.0)) (struct :`Roll` 90.0) true))))

(fn `GetInteractPrompt`
  (params (HitResult :type "HitResult Structure"))
  (returns (ReturnValue :type Text))
  (return "Missing book"))

(fn `UserConstructionScript`)